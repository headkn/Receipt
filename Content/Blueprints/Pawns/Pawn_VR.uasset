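; VR pawn that sets a floor-level tracking origin and provides thumbstick locomotion and snap turning.
; The left stick moves the actor without sweep along the camera's flattened forward and right vectors, scaled by Speed and delta time, with forward negated.
; The right stick yaws the actor in fixed steps, negative for positive input and vice versa, using latch flags that reset when the stick re-centers.
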(event EventBeginPlay
  (Class|HeadMountedDisplayFunctionLibrary|SetTrackingOrigin "Floor")
  (Input|EnableInput (Game|GetPlayerController 0)))

(event Collision|EventActorBeginOverlap
  (params (OtherActor :type Actor%20Object%20Reference)))

(event EventTick
  (params (DeltaSeconds :type Float%20%28single-precision%29)))

(event Input|KeyboardEvents|MotionControllerLeftThumbstickY
  (params (AxisValue :type Float%20%28single-precision%29))
  (Transformation|SetActorLocation (+ (Transformation|GetActorLocation) (* (* (Math|Vector|GetForwardVector (Transformation|GetWorldRotation (Variables|Default|GetCamera))) "-1.000000,-1.000000, 0") (* (Utilities|Time|GetWorldDeltaSeconds) AxisValue (Variables|Default|GetSpeed)))) false false))

(event Input|KeyboardEvents|MotionControllerLeftThumbstickX
  (params (AxisValue :type Float%20%28single-precision%29))
  (Transformation|SetActorLocation (+ (Transformation|GetActorLocation) (* (* (Math|Vector|GetRightVector (Transformation|GetWorldRotation (Variables|Default|GetCamera))) "1.000000,1.000000, 0") (* (Utilities|Time|GetWorldDeltaSeconds) AxisValue (Variables|Default|GetSpeed)))) false false))

(event Input|KeyboardEvents|MotionControllerRightThumbstickX
  (params (AxisValue :type Float%20%28single-precision%29))
  (bind _returnvalue (Transformation|GetActorRotation))
  (bind _returnvalue_2 (Transformation|GetActorRotation))
  (bind (_roll _pitch _yaw) (Math|Rotator|BreakRotator _returnvalue))
  (bind (_roll_2 _pitch_2 _yaw_2) (Math|Rotator|BreakRotator _returnvalue_2))
  (if (> AxisValue 0.8)
    (if (not (Variables|Default|GetIsRotatedLeft))
      (Variables|Default|SetIsRotatedLeft true)
      (Transformation|SetActorRotation (Math|Rotator|MakeRotator _roll_2 _pitch_2 (+ _yaw_2 -3e+01))))
    (elif (< AxisValue -0.8)
      (if (not (Variables|Default|GetIsRotatedRight))
        (Variables|Default|SetIsRotatedRight true)
        (Transformation|SetActorRotation (Math|Rotator|MakeRotator _roll _pitch (+ _yaw 3e+01))))
      (else
        (Variables|Default|SetIsRotatedLeft false)
        (Variables|Default|SetIsRotatedRight false)))))

(fn ConstructionScript)