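; BP_Btn is a button actor that gives visual press feedback by tinting its static mesh.
; The construction script creates a dynamic material instance from SourceMaterial on the mesh's first slot and stores it in Material.
; BtnClicked darkens the Color parameter to light grey and BtnReleased restores it to white.
; The file contains no input or click binding, and BeginPlay, overlap and Tick are empty.
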(event Custom|BtnClicked
  (Rendering|Material|SetVectorParameterValue (Variables|Default|GetMaterial) "Color" "(R=0.800000,G=0.800000,B=0.800000,A=1.000000)" :!class /Script/Engine.MaterialInstanceDynamic))

(event Custom|BtnReleased
  (Rendering|Material|SetVectorParameterValue (Variables|Default|GetMaterial) "Color" "(R=1.000000,G=1.000000,B=1.000000,A=1.000000)" :!class /Script/Engine.MaterialInstanceDynamic))

(event EventBeginPlay)

(event Collision|EventActorBeginOverlap
  (params (OtherActor :type Actor%20Object%20Reference)))

(event EventTick
  (params (DeltaSeconds :type Float%20%28single-precision%29)))

(fn ConstructionScript
  (bind _returnvalue (Rendering|Material|CreateDynamicMaterialInstance (Variables|Default|GetStaticMesh) 0 (Variables|Default|GetSourceMaterial) :!class /Script/Engine.PrimitiveComponent))
  (bind _output_get (Variables|Default|SetMaterial _returnvalue))
  (Rendering|Material|SetMaterial (Variables|Default|GetStaticMesh) 0 _output_get))