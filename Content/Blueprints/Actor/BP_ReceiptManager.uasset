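; BP_ReceiptManager is an actor that populates the level with a thousand BP_Receipt actors at BeginPlay.
; It finds the first Pawn_VR, passes it to each spawned receipt as Player, and stores the receipts in an array.
; GetRandomTransform uses a random stream and spherical-coordinate math to scatter them around the world origin between inner and outer radii, with the polar angle limited away from the poles.
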(event Custom|GenerateRandomReceipt
  (bind _transform (CallFunction|GetRandomTransform))
  (bind _returnvalue (Game|SpawnActorfromClass "/Game/Blueprints/Actor/BP_Receipt.BP_Receipt_C" _transform "Undefined" 0 0))
  (Variables|/Game/Blueprints/Actor/BP_Receipt.BP_Receipt_C|SetPlayer _returnvalue (Variables|Default|GetPlayer))
  (Utilities|Array|Add (Variables|Default|GetReceipts) _returnvalue))

(event Custom|GenerateReceipts
  (params (ReceiptNum :type Integer))
  (for _index (range 0 (- ReceiptNum 1))
    (CallFunction|GenerateRandomReceipt)))

(event EventBeginPlay
  (bind _outactors (Actor|GetAllActorsOfClass "/Game/Blueprints/Pawns/Pawn_VR.Pawn_VR_C"))
  (Variables|Default|SetPlayer (Utilities|Array|Get(acopy) _outactors))
  (CallFunction|GenerateReceipts 1000))

(event Collision|EventActorBeginOverlap
  (params (OtherActor :type Actor%20Object%20Reference)))

(event EventTick
  (params (DeltaSeconds :type Float%20%28single-precision%29)))

(fn ConstructionScript)

(fn GetRandomTransform
  (bind _randomstream (Variables|Default|GetRandomStream))
  (bind _randomstream_2 (Variables|Default|GetRandomStream))
  (bind _randomstream_3 (Variables|Default|GetRandomStream))
  (bind _innerrange (LocalVariables|GetInnerRange))
  (bind _outerrange (LocalVariables|GetOuterRange))
  (bind _returnvalue (Math|Random|RandomFloatinRangefromStream 0.0 3.6e+02 _randomstream_2))
  (bind _returnvalue_2 (Math|Random|RandomFloatinRangefromStream _innerrange _outerrange _randomstream_3))
  (bind _returnvalue_3 (Math|Random|RandomFloatinRangefromStream 3e+01 1.5e+02 _randomstream))
  (bind _returnvalue_4 (Math|Trig|Sin(Degrees) _returnvalue_3))
  (return (Math|Transform|MakeTransform (Math|Vector|MakeVector (* _returnvalue_2 _returnvalue_4 (Math|Trig|Cos(Degrees) _returnvalue)) (* _returnvalue_2 _returnvalue_4 (Math|Trig|Sin(Degrees) _returnvalue)) (* _returnvalue_2 (Math|Trig|Cos(Degrees) _returnvalue_3))))))