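; BP_Btn_Search is a button actor that shows or hides a child actor of a menu, presumably a search panel given the asset's name.
; On BtnClicked it runs the parent logic, then checks whether the Menu's ChildActor4 component is visible.
; It flips both visibility and hidden-in-game on that component, without propagating to its children.
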(event EventBeginPlay
  (|CallParentFunction) ; 지금 이 노드는 비활성 상태입니다. \n핀을 끌어서 다른 노드를 연결하면 활성화됩니다.
)

(event Collision|EventActorBeginOverlap
  (params (OtherActor :type Actor%20Object%20Reference))
  (|CallParentFunction OtherActor) ; 지금 이 노드는 비활성 상태입니다. \n핀을 끌어서 다른 노드를 연결하면 활성화됩니다.
)

(event EventBtnClicked
  (bind _menu (Variables|Default|GetMenu))
  (bind _childactor4 (Variables|/Game/Blueprints/Actor/BP_Menu.BP_Menu_C|GetChildActor4 _menu))
  (|CallParentFunction)
  (if (Rendering|IsVisible _childactor4)
    (Rendering|SetVisibility _childactor4 false false)
    (Development|SetHiddeninGame _childactor4 true false)
    (else
      (Rendering|SetVisibility _childactor4 true false)
      (Development|SetHiddeninGame _childactor4 false false))))

(event EventTick
  (params (DeltaSeconds :type Float%20%28single-precision%29))
  (|CallParentFunction DeltaSeconds) ; 지금 이 노드는 비활성 상태입니다. \n핀을 끌어서 다른 노드를 연결하면 활성화됩니다.
)

(fn ConstructionScript
  (|CallParentFunction))