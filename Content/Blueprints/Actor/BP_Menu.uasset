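; BP_Menu is a menu actor that hosts four BP_Btn buttons as child actors and connects them to the receipt manager.
; On BeginPlay it finds the first BP_ReceiptManager in the level with GetAllActorsOfClass.
; It then casts each child actor to BP_Btn and injects both that manager and itself as references.
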(event EventBeginPlay
  (Utilities|FlowControl|Sequence
    (:then_0
      (bind _outactors (Actor|GetAllActorsOfClass "/Game/Blueprints/Actor/BP_ReceiptManager.BP_ReceiptManager_C"))
      (Variables|Default|SetReceiptManager (Utilities|Array|Get(acopy) _outactors)))
    (:then_1
      (bind _asbp_btn (Utilities|Casting|CastToBP_Btn (Variables|/Script/Engine.ChildActorComponent|GetChildActor (Variables|Default|GetChildActor))))
      (Variables|/Game/Blueprints/Actor/BP_Btn.BP_Btn_C|SetReceiptManager _asbp_btn (Variables|Default|GetReceiptManager))
      (Variables|/Game/Blueprints/Actor/BP_Btn.BP_Btn_C|SetMenu _asbp_btn self))
    (:then_2
      (bind _asbp_btn_2 (Utilities|Casting|CastToBP_Btn (Variables|/Script/Engine.ChildActorComponent|GetChildActor (Variables|Default|GetChildActor1))))
      (Variables|/Game/Blueprints/Actor/BP_Btn.BP_Btn_C|SetReceiptManager _asbp_btn_2 (Variables|Default|GetReceiptManager))
      (Variables|/Game/Blueprints/Actor/BP_Btn.BP_Btn_C|SetMenu _asbp_btn_2 self))
    (:then_3
      (bind _asbp_btn_3 (Utilities|Casting|CastToBP_Btn (Variables|/Script/Engine.ChildActorComponent|GetChildActor (Variables|Default|GetChildActor2))))
      (Variables|/Game/Blueprints/Actor/BP_Btn.BP_Btn_C|SetReceiptManager _asbp_btn_3 (Variables|Default|GetReceiptManager))
      (Variables|/Game/Blueprints/Actor/BP_Btn.BP_Btn_C|SetMenu _asbp_btn_3 self))
    (:then_4
      (bind _asbp_btn_4 (Utilities|Casting|CastToBP_Btn (Variables|/Script/Engine.ChildActorComponent|GetChildActor (Variables|Default|GetChildActor3))))
      (Variables|/Game/Blueprints/Actor/BP_Btn.BP_Btn_C|SetReceiptManager _asbp_btn_4 (Variables|Default|GetReceiptManager))
      (Variables|/Game/Blueprints/Actor/BP_Btn.BP_Btn_C|SetMenu _asbp_btn_4 self))))

(event Collision|EventActorBeginOverlap
  (params (OtherActor :type Actor%20Object%20Reference)))

(event EventTick
  (params (DeltaSeconds :type Float%20%28single-precision%29)))

(fn ConstructionScript)