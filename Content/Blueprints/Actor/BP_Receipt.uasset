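; BP_Receipt is a receipt actor that can be held by a hand component and otherwise stands in place facing the player.
; The construction script randomizes Plane's color material and Plane1's image, using the image index to choose Plane's scale.
; Tick pins it, shrunk, in front of GrabbedHand while valid, otherwise snapping it back to its BeginPlay location at full scale.
; GrabbedHand is not assigned in these graphs.
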(event EventBeginPlay
  (Variables|Default|SetInitialPosition (Transformation|GetActorLocation)))

(event Collision|EventActorBeginOverlap
  (params (OtherActor :type Actor%20Object%20Reference)))

(event EventTick
  (params (DeltaSeconds :type Float%20%28single-precision%29))
  (bind _grabbedhand (Variables|Default|GetGrabbedHand))
  (bind _returnvalue (Transformation|GetWorldRotation _grabbedhand))
  (Utilities|IsValid (Variables|Default|GetGrabbedHand)
    (:Is%20Valid
      (Transformation|SetActorTransform (Math|Transform|MakeTransform (+ (Transformation|GetWorldLocation (Variables|Default|GetGrabbedHand)) (* (Math|Vector|GetForwardVector _returnvalue) 2e+01)) _returnvalue "0.100000,0.100000,0.100000")))
    (:Is%20Not%20Valid
      (Transformation|SetActorTransform (Math|Transform|MakeTransform (Variables|Default|GetInitialPosition) (Math|Rotator|MakeRotfromXZ (Math|Vector|MakeVector 0.0 0.0 1.0) (- (Transformation|GetActorLocation (Variables|Default|GetPlayer)) (Transformation|GetActorLocation))))))))

(fn ConstructionScript
  (Rendering|Material|SetMaterial (Variables|Default|GetPlane) 0 (Utilities|Array|Get(acopy) (LocalVariables|GetColorRandomMaterial) (Math|Random|RandomIntegerinRange 0 7)))
  (LocalVariables|SetImageRandomInteger (Math|Random|RandomIntegerinRange 0 3))
  (Rendering|Material|SetMaterial (Variables|Default|GetPlane1) 0 (Utilities|Array|Get(acopy) (LocalVariables|GetImageRandomMaterial) (LocalVariables|GetImageRandomInteger)))
  (Transformation|SetRelativeScale3D (Variables|Default|GetPlane) (Utilities|Array|Get(acopy) (LocalVariables|GetScaleRandomVector) (LocalVariables|GetImageRandomInteger))))